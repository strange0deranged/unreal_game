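; Player character for a 2D flipbook platformer, with jumping, side-to-side movement and an interact action through Enhanced Input.
; Movement input runs along world X and flips the control rotation yaw to face the travel direction.
; Tick picks idle, walk, jump or fall flipbooks from ground state and velocity, and pins the widget's world rotation.
; Capsule overlaps track nearby Interactable or Exit actors, so interact shows message text or opens the exit's level.
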(event OnComponentEndOverlap(CapsuleComponent)
  (params (OverlappedComponent :type Primitive%20Component%20Object%20Reference) (OtherActor :type Actor%20Object%20Reference) (OtherComp :type Primitive%20Component%20Object%20Reference) (OtherBodyIndex :type Integer))
  (Utilities|Casting|CastToInteractable OtherActor
    (:then
      (Variables|Default|SetisInteractable false)
      (bind _asmy_message_widget (Utilities|Casting|CastToMyMessageWidget (UserInterface|GetWidget (Variables|Default|GetWidget))))
      (Variables|/Game/Assets/blueprints/MyMessageWidget.MyMessageWidget_C|SetText _asmy_message_widget ""))
    (:CastFailed
      (Utilities|Casting|CastToExit OtherActor)
      (Variables|Default|SetisExit false))))

(event OnComponentBeginOverlap(CapsuleComponent)
  (params (OverlappedComponent :type Primitive%20Component%20Object%20Reference) (OtherActor :type Actor%20Object%20Reference) (OtherComp :type Primitive%20Component%20Object%20Reference) (OtherBodyIndex :type Integer) (bFromSweep :type Boolean) (SweepResult :type Hit%20Result%20Structure%20%28by%20ref%29))
  (bind _asinteractable (Utilities|Casting|CastToInteractable OtherActor)
    (:then
      (Variables|Default|SetisInteractable true)
      (Variables|Default|SetInteractable _asinteractable))
    (:CastFailed
      (bind _asexit (Utilities|Casting|CastToExit OtherActor))
      (Variables|Default|SetisExit true)
      (Variables|Default|SetExit _asexit))))

(event Input|EnhancedActionEvents|EnhancedInputActionjump
  (params (ActionValue :type Boolean) (ElapsedSeconds :type Float%20%28double-precision%29) (TriggeredSeconds :type Float%20%28double-precision%29) (InputAction :type Input%20Action%20Object%20Reference :default "/Game/Assets/input/actions/jump.jump"))
  (:Started
    (Character|Jump))
  (:Completed
    (Character|StopJumping)))

(event Input|EnhancedActionEvents|EnhancedInputActionmove
  (params (ActionValue :type Float%20%28double-precision%29) (ElapsedSeconds :type Float%20%28double-precision%29) (TriggeredSeconds :type Float%20%28double-precision%29) (InputAction :type Input%20Action%20Object%20Reference :default "/Game/Assets/input/actions/move.move"))
  (Pawn|Input|AddMovementInput "1.000000,0.000000,0.000000" ActionValue false)
  (Pawn|SetControlRotation (Pawn|GetController) (select (> ActionValue 0.0) (Math|Rotator|MakeRotator 0.0 0.0 0.0) (Math|Rotator|MakeRotator 0.0 0.0 1.8e+02))))

(event Input|EnhancedActionEvents|EnhancedInputActioninteract
  (params (ActionValue :type Boolean) (ElapsedSeconds :type Float%20%28double-precision%29) (TriggeredSeconds :type Float%20%28double-precision%29) (InputAction :type Input%20Action%20Object%20Reference :default "/Game/Assets/input/actions/interact.interact"))
  (:Started
    (if (Variables|Default|GetisExit)
      (Game|OpenLevel(byName) (Utilities|String|StringToName (Variables|/Game/Assets/blueprints/Exit.Exit_C|GetLevel (Variables|Default|GetExit))))
      (elif (Variables|Default|GetisInteractable)
        (bind _asmy_message_widget (Utilities|Casting|CastToMyMessageWidget (UserInterface|GetWidget (Variables|Default|GetWidget))))
        (Variables|/Game/Assets/blueprints/MyMessageWidget.MyMessageWidget_C|SetText _asmy_message_widget (Variables|/Game/Assets/blueprints/Interactable.Interactable_C|GetText (Variables|Default|GetInteractable)))))))

(event EventBeginPlay
  (Utilities|FlowControl|Sequence
    (:then_0
      (bind _asplayer_controller (Utilities|Casting|CastToPlayerController (Pawn|GetController)))
      (Input|AddMappingContext (PlayerController|LocalPlayerSubsystems|GetEnhancedInputLocalPlayerSubsystem _asplayer_controller) "/Game/Assets/input/platforming.platforming" 0 "(bIgnoreAllPressedKeysUntilRelease=True,bForceImmediately=False,bNotifyUserSettings=False)"))
    (:then_1
      (Variables|Default|SetisExit false)
      (Variables|Default|SetisInteractable false))))

(event Collision|EventActorBeginOverlap
  (params (OtherActor :type Actor%20Object%20Reference)))

(event EventTick
  (params (DeltaSeconds :type Float%20%28single-precision%29))
  (Utilities|FlowControl|Sequence
    (:then_0
      (CallFunction|UpdateAnimation))
    (:then_1
      (Transformation|SetWorldRotation (Variables|Default|GetWidget) "0.000000,90.000000,0.000000" false false))))

(fn ConstructionScript)

(fn UpdateAnimation
  (if (AI|Components|NavMovement|IsMovingonGround (Variables|Character|GetCharacterMovement))
    (if (> (Math|Vector|VectorLength (Transformation|GetVelocity)) 0.0)
      (Sprite|SetFlipbook (Variables|Default|GetSprite) "/Game/Assets/player/sprites/girl_walking_fix.girl_walking_fix")
      (else
        (Sprite|SetFlipbook (Variables|Default|GetSprite) "/Game/Assets/player/flipbooks/girl_idle.girl_idle")))
    (elif (> (.z (Transformation|GetVelocity)) -5e+01)
      (Sprite|SetFlipbook (Variables|Default|GetSprite) "/Game/Assets/player/flipbooks/girl_jump.girl_jump")
      (else
        (Sprite|SetFlipbook (Variables|Default|GetSprite) "/Game/Assets/player/flipbooks/girl_fall.girl_fall")))))