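; Exit actor, a 2D sprite that scales into view while something overlaps its trigger sprite.
; On play it hides the collision sprite and collapses the exit sprite to zero width and height.
; Overlap begin plays the In timeline to grow the sprite's X and Z scale, and overlap end reverses it.
; The construction script sizes the collision sprite from the Width and Height variables.
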(event OnComponentBeginOverlap(default_collision_Sprite)
  (params (OverlappedComponent :type Primitive%20Component%20Object%20Reference) (OtherActor :type Actor%20Object%20Reference) (OtherComp :type Primitive%20Component%20Object%20Reference) (OtherBodyIndex :type Integer) (bFromSweep :type Boolean) (SweepResult :type Hit%20Result%20Structure%20%28by%20ref%29))
  (bind _value (Timeline|In PlayFromStart)
    (:Update
      (Transformation|SetWorldScale3D (Variables|Default|Getexit_Sprite) (Math|Vector|MakeVector _value 1.0 _value)))))

(event OnComponentEndOverlap(default_collision_Sprite)
  (params (OverlappedComponent :type Primitive%20Component%20Object%20Reference) (OtherActor :type Actor%20Object%20Reference) (OtherComp :type Primitive%20Component%20Object%20Reference) (OtherBodyIndex :type Integer))
  (bind _value (Timeline|In Reverse)
    (:Update
      (Transformation|SetWorldScale3D (Variables|Default|Getexit_Sprite) (Math|Vector|MakeVector _value 1.0 _value)))))

(event EventBeginPlay
  (Rendering|SetVisibility (Variables|Default|Getdefault_collision_Sprite) false false)
  (Transformation|SetWorldScale3D (Variables|Default|Getexit_Sprite) "0.000000,1.000000,0.000000"))

(event Collision|EventActorBeginOverlap
  (params (OtherActor :type Actor%20Object%20Reference)))

(event EventTick
  (params (DeltaSeconds :type Float%20%28single-precision%29)))

(fn ConstructionScript
  (Transformation|SetRelativeScale3D (Variables|Default|Getdefault_collision_Sprite) (Math|Vector|MakeVector (Variables|Components|GetWidth) 1.0 (Variables|Components|GetHeight))))