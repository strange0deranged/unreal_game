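; A side-scrolling camera Blueprint that follows the player character horizontally while staying within the level's bounds.
; BeginPlay derives left and right limits from hard-coded level and camera widths, insetting each edge by half the camera width.
; Every Tick, it moves its scene component to the player's X clamped between those limits, with Y and Z held fixed and no smoothing.
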(event EventBeginPlay
  (bind _output_get (Variables|Default|SetLevelWidth 3918.0))
  (bind _output_get_2 (Variables|Default|SetCameraWidth 2388.0))
  (bind _output_get_3 (Variables|Default|SetLeftBoundary (/ _output_get_2 2.0)))
  (Variables|Default|SetRightBoundary (- _output_get _output_get_3)))

(event Collision|EventActorBeginOverlap
  (params (OtherActor :type Actor%20Object%20Reference)))

(event EventTick
  (params (DeltaSeconds :type Float%20%28single-precision%29))
  (Transformation|SetWorldLocation (Variables|Default|GetSceneComponent) (Math|Vector|MakeVector (Math|Float|Clamp(Float) (.X (Math|Vector|BreakVector (Transformation|GetActorLocation (Game|GetPlayerCharacter 0)))) (Variables|Default|GetLeftBoundary) (Variables|Default|GetRightBoundary)) -1e+01 0.0) false false))

(fn ConstructionScript)